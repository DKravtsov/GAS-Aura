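; Fire ball actor for Aura's FireBlast ability, with movement logic that is not wired up in this graph.
; BeginPlay caches the instigator's location and computes a target MaxDistance along the actor's forward vector.
; An unconnected timeline lerps from the instigator's current location to that target.
; UpdateFireBallLocation interpolates back toward the instigator, facing the instigator's movement delta, but its only call here is unconnected.
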(event `self.ReceiveBeginPlay`
  (bind _output_get (set `self.LastAuraLocation` (`self.K2_GetActorLocation` (`self.GetInstigator`))))
  (bind _output_get_2 (set `self.InitialLocation` _output_get))
  (set `self.TargetLocation` (+ _output_get_2 (* (`self.GetActorForwardVector`) (`self.MaxDistance`)))))

(fn `UpdateFireBallLocation`
  (params (DeltaTime :type "Float (single-precision)"))
  (locals (CurrentLocation :type "Vector Structure") (LocationDelta :type "Vector Structure"))
  (set `local.CurrentLocation` (`self.K2_GetActorLocation` (`self.GetInstigator`)))
  (set `local.LocationDelta` (- (`local.CurrentLocation`) (`self.LastAuraLocation`)))
  (set `self.LastAuraLocation` (`local.CurrentLocation`))
  (`self.K2_SetActorLocationAndRotation` (`KismetMathLibrary.VInterpTo` (`self.K2_GetActorLocation`) (`local.CurrentLocation`) (`local.DeltaTime`) 2.0) (`KismetMathLibrary.MakeRotFromX` (`local.LocationDelta`))))

(fn `UserConstructionScript`)