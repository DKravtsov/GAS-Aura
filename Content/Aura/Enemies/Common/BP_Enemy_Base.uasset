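; Base enemy Blueprint providing death dissolve, attack-facing and health widget access.
; DissolveDeadBody creates dynamic materials for mesh and weapon, opening a gate so one timeline drives their Dissolve parameter if either material is valid.
; UpdateFacingTarget sets the FacingTarget motion warp location, and GetHealthOverlayWidget returns the overlay component's widget as AuraUserWidget.
; A spawn scale timeline exists but is never triggered.
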(event `self.ReceiveBeginPlay`)

(event `self.DissolveDeadBody`
  (`|ExecutionSequence`
    (:`then_0`
      (bind _disolvematerial (`self.DisolveMaterial`)
        (:`then`
          (bind _returnvalue (`PrimitiveComponent.CreateDynamicMaterialInstance` (`self.Mesh`) 0 _disolvematerial "None"))
          (set `self.MeshDynamicMatInst` _returnvalue)
          (goto _label :!via `Open`))
        (:`else`)))
    (:`then_1`
      (bind _weapondisolvematerial (`self.WeaponDisolveMaterial`)
        (:`then`
          (bind _returnvalue_2 (`PrimitiveComponent.CreateDynamicMaterialInstance` (`self.Weapon`) 0 _weapondisolvematerial "None"))
          (set `self.WeaponDynamicMatInst` _returnvalue_2)
          (goto _label :!via `Open`))
        (:`else`)))
    (:`then_2`
      (`/Engine/EditorBlueprintResources/StandardMacros.Gate` true :!label _label
        (:`Exit`
          (bind (_direction _disolvealpha) (`Timeline|Timeline_Disolve`)
            (:`Update`
              (`self.SetDissolveParam` _disolvealpha))))))))

(event `CombatInterface.UpdateFacingTarget`
  (params (TargetLocation :type "Vector Structure (by ref)"))
  (`MotionWarpingComponent.AddOrUpdateWarpTargetFromLocation` (`self.MotionWarping`) "FacingTarget" TargetLocation))

(fn `GetHealthOverlayWidget`
  (returns (ReturnValue :type "AuraUserWidget Object Reference"))
  (bind _asaura_user_widget (cast `AuraUserWidget` (`WidgetComponent.GetUserWidgetObject` (`self.OverlayWidgetComponent`))))
  (return _asaura_user_widget))

(fn `UserConstructionScript`)