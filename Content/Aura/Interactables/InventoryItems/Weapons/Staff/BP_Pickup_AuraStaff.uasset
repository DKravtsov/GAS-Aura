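; Aura staff weapon pickup that spins in the world and can be highlighted.
; Tick adds a fixed local rotation to the mesh each frame, unscaled by delta time, so spin speed follows frame rate.
; Two pairs of highlight events share logic that applies or clears an outline overlay material on the mesh.
; GetMoveToDestination returns the actor's own location as the move target.
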(event `self.ReceiveTick`
  (params (DeltaSeconds :type "Float (single-precision)"))
  (`SceneComponent.K2_AddLocalRotation` (`self.Mesh`) (struct :`Yaw` 2.0) false false))

(event `InventoryHighlightableInterface.Highlight`
  (`MeshComponent.SetOverlayMaterial` (`self.Mesh`) (`self.OutlineMaterial`) :!label _label))

(event `InteractableInterface.HighlightActor`
  (goto _label))

(event `InventoryHighlightableInterface.UnHighlight`
  (`MeshComponent.SetOverlayMaterial` (`self.Mesh`) null :!label _label_2))

(event `InteractableInterface.UnhighlightActor`
  (goto _label_2))

(fn `GetMoveToDestination`
  (returns (OutDestination :type "Vector Structure"))
  (return (`self.K2_GetActorLocation`)))

(fn `UserConstructionScript`)