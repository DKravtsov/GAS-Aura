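; BP_Pickup_Base is the base pickup actor, handling spawn animation, idle motion and sounds for pickups.
; On BeginPlay it plays the spawn sound and runs a startup timeline that drives mesh height and scales it relative to its initial size.
; A Ground Hit event track triggers the impact sound, and on finish a slowed movement timeline takes over height and yaw.
; Destruction plays the consume sound.
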(event `self.ReceiveBeginPlay`
  (bind _staticmesh (`self.StaticMesh`))
  (`TimelineComponent.SetPlayRate` (`self.Timeline_Movement`) 0.18)
  (`GameplayStatics.PlaySoundAtLocation` (`self.SpawnSound`) (`self.K2_GetActorLocation`) (struct) 1.0 1.0 0.0 null null null null)
  (set `self.InitialScale` (`SceneComponent.K2_GetComponentScale` (`self.StaticMesh`)))
  (bind (_direction _height _scale) (`Timeline|Timeline_Startup`)
    (:`Update`
      (`SceneComponent.K2_SetRelativeLocation` _staticmesh (`KismetMathLibrary.MakeVector` 0.0 0.0 _height) false false)
      (`SceneComponent.SetWorldScale3D` _staticmesh (* (`self.InitialScale`) _scale)))
    (:`Finished`
      (bind (_direction_2 _height_2 _rotationangle) (`Timeline|Timeline_Movement` :!via `PlayFromStart`)
        (:`Update`
          (`SceneComponent.K2_SetRelativeLocationAndRotation` (`self.StaticMesh`) (`KismetMathLibrary.MakeVector` 0.0 0.0 _height_2) (`KismetMathLibrary.MakeRotator` 0.0 0.0 _rotationangle) false false))))
    (:`GroundHit`
      (`GameplayStatics.PlaySoundAtLocation` (`self.GroundImpactSound`) (`self.K2_GetActorLocation`) (struct) 1.0 1.0 0.0 null null null null))))

(event `self.ReceiveDestroyed`
  (`GameplayStatics.PlaySoundAtLocation` (`self.ConsumeSound`) (`self.K2_GetActorLocation`) (struct) 1.0 1.0 0.0 null null null null))

(fn `UserConstructionScript`)