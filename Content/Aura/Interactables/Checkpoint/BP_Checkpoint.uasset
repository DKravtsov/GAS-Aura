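; BP_Checkpoint is an interactable checkpoint that shows its reached state by making its mesh glow.
; When the checkpoint-reached event fires with CheckpointReached set, it creates a dynamic instance of the mesh's first material and plays Timeline_Glowing to drive the scaled Glow parameter.
; When the flag is cleared and that instance exists, the timeline reverses from its end.
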(event `self.ReceivedCheckpointReached`
  (bind _checkpointmesh (`self.CheckpointMesh`))
  (if (`self.bCheckpointReached`)
    (bind _returnvalue (`PrimitiveComponent.CreateDynamicMaterialInstance` _checkpointmesh 0 (`PrimitiveComponent.GetMaterial` _checkpointmesh 0) "None"))
    (set `self.DynamicMat` _returnvalue)
    (bind (_direction _alpha) (`Timeline|Timeline_Glowing` :!label _label)
      (:`Update`
        (`MaterialInstanceDynamic.SetScalarParameterValue` (`self.DynamicMat`) "Glow" (* _alpha 80.0))))
    (else
      (`self.DynamicMat`
        (:`then`
          (goto _label :!via `ReverseFromEnd`))
        (:`else`)))))

(fn `UserConstructionScript`)