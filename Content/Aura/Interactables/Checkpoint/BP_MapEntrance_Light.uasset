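; BP_MapEntrance_Light is a map entrance interactable whose two point lights act as its highlight feedback.
; It hides both lights on BeginPlay, shows them on HighlightActor and hides them again on UnhighlightActor.
; BeginPlay and the construction script call their parent versions, and Tick is disabled.
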(event `self.ReceiveBeginPlay`
  (`parent.ReceiveBeginPlay`)
  (`SceneComponent.SetVisibility` (`self.PointLight`) false false)
  (`SceneComponent.SetVisibility` (`self.PointLight1`) false false))

(event `InteractableInterface.HighlightActor`
  (`SceneComponent.SetVisibility` (`self.PointLight`) true false)
  (`SceneComponent.SetVisibility` (`self.PointLight1`) true false))

(event `InteractableInterface.UnhighlightActor`
  (`SceneComponent.SetVisibility` (`self.PointLight`) false false)
  (`SceneComponent.SetVisibility` (`self.PointLight1`) false false))

(fn `UserConstructionScript`
  (`parent.UserConstructionScript`))