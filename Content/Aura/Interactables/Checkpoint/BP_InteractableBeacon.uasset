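; BP_InteractableBeacon is a checkpoint beacon that activates when an actor implementing PlayerInterface overlaps its box.
; Activation disables box collision, sets CheckpointReached and drives a dynamic material's Glow through a timeline.
; Loading from a save replays activation if already reached, without restoring the transform.
; It highlights through custom depth stencil only while unreached and supplies TargetDest's location as the move-to destination.
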(event `InteractableInterface.HighlightActor`
  (bind _staticmeshcomponent (`self.StaticMeshComponent`))
  (if (not (`self.bCheckpointReached`))
    (`PrimitiveComponent.SetRenderCustomDepth` _staticmeshcomponent true)
    (`PrimitiveComponent.SetCustomDepthStencilValue` _staticmeshcomponent 252)))

(event `InteractableInterface.UnhighlightActor`
  (`PrimitiveComponent.SetRenderCustomDepth` (`self.StaticMeshComponent`) false))

(event `self.Box.OnComponentBeginOverlap`
  (params (OverlappedComponent :type "PrimitiveComponent Object Reference") (OtherActor :type "Actor Object Reference") (OtherComp :type "PrimitiveComponent Object Reference") (OtherBodyIndex :type Integer) (bFromSweep :type Boolean) (SweepResult :type "HitResult Structure (by ref)"))
  (if (`KismetSystemLibrary.DoesImplementInterface` OtherActor "/Script/Aura.PlayerInterface")
    (`self.CheckpointReached`)))

(event `CheckpointReached`
  (bind _staticmeshcomponent (`self.StaticMeshComponent`))
  (`PrimitiveComponent.SetCollisionEnabled` (`self.Box`) "NoCollision")
  (set `self.bCheckpointReached` true)
  (bind _returnvalue (`PrimitiveComponent.CreateDynamicMaterialInstance` _staticmeshcomponent 0 (`PrimitiveComponent.GetMaterial` _staticmeshcomponent 0) "None"))
  (set `self.DynamicMat` _returnvalue)
  (bind (_direction _alpha) (`Timeline|Timeline`)
    (:`Update`
      (`MaterialInstanceDynamic.SetScalarParameterValue` (`self.DynamicMat`) "Glow" (* _alpha 100.0)))))

(event `SaveGameInterface.LoadedFromSaveGame`
  (if (`self.bCheckpointReached`)
    (`self.CheckpointReached`)))

(fn `GetMoveToDestination`
  (returns (OutDestination :type "Vector Structure"))
  (return (`SceneComponent.K2_GetComponentLocation` (`self.TargetDest`))))

(fn `ShouldLoadTransform`
  (returns (ReturnValue :type Boolean))
  (return false))

(fn `UserConstructionScript`)