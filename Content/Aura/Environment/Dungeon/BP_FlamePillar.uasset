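; BP_FlamePillar is a dungeon environment flame pillar whose FireLight flickers through randomized intensity animation.
; Each cycle randomly picks one of two timelines, varies its play rate and multiplies its curve by BaseIntensity to drive the light.
; When either timeline finishes, the Play event starts a new random cycle, giving an endless, irregular flicker.
; The construction script applies BaseIntensity to the light as its initial brightness.
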(event `self.ReceiveBeginPlay`
  (bind _returnvalue (+ 1.0 (`KismetMathLibrary.RandomFloatInRange` -0.2 0.35)))
  (if (`KismetMathLibrary.RandomBool`) :!label _label
    (`TimelineComponent.SetPlayRate` (`self.Timeline_Intensity`) _returnvalue)
    (bind (_direction _intensity) (`Timeline|Timeline_Intensity` :!via `PlayFromStart`)
      (:`Update`
        (`LightComponent.SetIntensity` (`self.FireLight`) (* _intensity (`self.BaseIntensity`))))
      (:`Finished`
        (`self.Play` :!label _label_2)))
    (else
      (`TimelineComponent.SetPlayRate` (`self.Timeline_Intensicty2`) _returnvalue)
      (bind (_direction_2 _intencity_2) (`Timeline|Timeline_Intensicty2` :!via `PlayFromStart`)
        (:`Update`
          (`LightComponent.SetIntensity` (`self.FireLight`) (* _intencity_2 (`self.BaseIntensity`))))
        (:`Finished`
          (goto _label_2))))))

(event `Play`
  (goto _label))

(fn `UserConstructionScript`
  (`LightComponent.SetIntensity` (`self.FireLight`) (`self.BaseIntensity`)))