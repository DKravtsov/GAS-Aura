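; BP_FadeActor is an environment actor whose static mesh fades out and back in through FadeOut and Fadein events.
; The construction script caches original materials and creates dynamic instances from FadeMaterials.
; FadeOut swaps those instances in and plays a timeline driving their Fade parameter, which Fadein reverses.
; On finish, alpha at one restores original materials and blocks the Visibility channel; otherwise the mesh ignores it.
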(event `self.ReceiveBeginPlay`)

(event `/Game/Aura/Environment/FadeActor/BPI_FadeInterface.FadeOut`
  (`self.SetMaterialsToDynamicInstances`)
  (bind (_direction _alpha) (`Timeline|Timeline_Fade` :!label _label)
    (:`Update`
      (for _array_element (`self.DynamicMaterials`)
        (`MaterialInstanceDynamic.SetScalarParameterValue` _array_element "Fade" _alpha)))
    (:`Finished`
      (`self.FadeFinished` _alpha))))

(event `/Game/Aura/Environment/FadeActor/BPI_FadeInterface.FadeIn`
  (goto _label :!via `Reverse`))

(fn `FadeFinished`
  (params (A :type "Float (double-precision)"))
  (if (>= A 1.0)
    (`self.ResetMaterials`)
    (`PrimitiveComponent.SetCollisionResponseToChannel` (`self.StaticMesh`) "ECC_Visibility" "ECR_Block")
    (else
      (`PrimitiveComponent.SetCollisionResponseToChannel` (`self.StaticMesh`) "ECC_Visibility" "ECR_Ignore"))))

(fn `ResetMaterials`
  (for (_array_element _array_index) (`self.OriginalMaterials`)
    (`PrimitiveComponent.SetMaterial` (`self.StaticMesh`) _array_index _array_element)))

(fn `SetMaterialsToDynamicInstances`
  (for (_array_element _array_index) (`self.DynamicMaterials`)
    (`PrimitiveComponent.SetMaterial` (`self.StaticMesh`) _array_index _array_element)))

(fn `UserConstructionScript`
  (`KismetArrayLibrary.Array_Clear` (`self.DynamicMaterials`))
  (set `self.OriginalMaterials` (`MeshComponent.GetMaterials` (`self.StaticMesh`)))
  (for _array_element (`self.FadeMaterials`)
    (bind _returnvalue (`KismetMaterialLibrary.CreateDynamicMaterialInstance` _array_element))
    (`KismetArrayLibrary.Array_AddUnique` (`self.DynamicMaterials`) _returnvalue)))