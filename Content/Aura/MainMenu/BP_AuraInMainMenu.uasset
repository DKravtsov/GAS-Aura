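; BP_AuraInMainMenu is the main menu actor, which animates a floating fireball and starts up the menu.
; BeginPlay caches the fireball's location, starts the menu music, creates and shows WBP_MainMenu, and enables the mouse cursor with UI-only input.
; Tick bobs the fireball vertically around that location with a sine wave, using a time accumulator that UpdateTime resets after passing two pi.
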(event `self.ReceiveBeginPlay`
  (bind _returnvalue (`GameplayStatics.GetPlayerController` 0))
  (set `self.InitialLocation` (`SceneComponent.K2_GetComponentLocation` (`self.Fireball`)))
  (bind _returnvalue_2 (`GameplayStatics.SpawnSound2D` "/Game/Assets/Sounds/Music/Music_MainMenu.Music_MainMenu" 1.0 1.0 0.0 null))
  (set `self.MainMenuMusic` _returnvalue_2)
  (bind _returnvalue_3 (`|CreateWidget` "/Game/Aura/MainMenu/WBP_MainMenu.WBP_MainMenu_C"))
  (`UserWidget.AddToViewport` _returnvalue_3 0)
  (set `PlayerController.bShowMouseCursor` true _returnvalue)
  (`WidgetBlueprintLibrary.SetInputMode_UIOnlyEx` _returnvalue null))

(event `self.ReceiveTick`
  (params (DeltaSeconds :type "Float (single-precision)"))
  (`self.UpdateTime` DeltaSeconds)
  (`SceneComponent.K2_SetWorldLocation` (`self.Fireball`) (+ (`self.InitialLocation`) (`KismetMathLibrary.MakeVector` 0.0 0.0 (* (`KismetMathLibrary.Sin` (`self.Time`)) (`self.Amplitude`)))) false false))

(fn `UpdateTime`
  (params (DeltaSeconds :type "Float (double-precision)"))
  (bind _output_get (set `self.Time` (+ DeltaSeconds (`self.Time`))))
  (if (> _output_get (`KismetMathLibrary.MultiplyByPi` 2.0))
    (set `self.Time` 0.0)))

(fn `UserConstructionScript`)